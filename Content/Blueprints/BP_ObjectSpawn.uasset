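; Item spawner actor that spawns a random class from its Objects array on BeginPlay.
; Shortly after spawning, it asks BP_GameInstance whether its ActorID was destroyed and, if so, destroys itself.
; With Respawn on, a BP_ThirdPersonCharacter entering the box records the pickup in the game instance, then the same class respawns after RespawnDelay.
; Several unconnected spawn experiments remain in the event graph.
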(event OnComponentBeginOverlap(BoxCollision)
  (params (OverlappedComponent :type Primitive%20Component%20Object%20Reference) (OtherActor :type Actor%20Object%20Reference) (OtherComp :type Primitive%20Component%20Object%20Reference) (OtherBodyIndex :type Integer) (bFromSweep :type Boolean) (SweepResult :type Hit%20Result%20Structure%20%28by%20ref%29))
  (bind _respawndelay (Variables|Default|GetRespawnDelay))
  ;[1 1 1] Respawning
  (if (Variables|Default|GetRespawn)
    (Utilities|Casting|CastToBP_ThirdPersonCharacter OtherActor)
    (CallFunction|PickUp)
    (Development|PrintString (Utilities|String|Append "Object Collected! Respawning in " (Utilities|String|ToString(Float) _respawndelay) " seconds") true true "(R=0.000000,G=0.660000,B=1.000000,A=1.000000)" _respawndelay)
    (Utilities|FlowControl|Delay (Variables|Default|GetRespawnDelay))
    (Game|SpawnActorfromClass (Variables|Default|GetSelectedObject) (Transformation|GetActorTransform (Components|GetOwner (Variables|Default|GetChildActor))) "Undefined" 0 0)
    (Development|PrintString "Created a copy object")
    (else
      (Development|PrintString "Respawn is off"))))

(event Custom|Pick%20Up
  (bind _asbp_game_instance (Utilities|Casting|CastToBP_GameInstance (Game|GetGameInstance)))
  (Default|DestroyItem _asbp_game_instance (Variables|Default|GetActor%20ID)))

(event EventBeginPlay
  (bind _objects (Variables|Default|GetObjects))
  (Utilities|FlowControl|Sequence
    (:then_0
      ;[1 1 1] Selecting an Object to Spawn
      (bind _output_get (Variables|Default|SetSelectedObject (Utilities|Array|Get(acopy) _objects (Math|Random|RandomInteger (Utilities|Array|Length _objects)))))
      ;[1 1 1] Spawning
      (Game|SpawnActorfromClass _output_get (Transformation|GetActorTransform (Components|GetOwner (Variables|Default|GetChildActor))) "Undefined" 0 0))
    (:then_1
      (Utilities|FlowControl|Delay 0.2)
      (bind _asbp_game_instance (Utilities|Casting|CastToBP_GameInstance (Game|GetGameInstance)))
      (bind _hasbeendestroyed (Default|CheckifDestroyed _asbp_game_instance (Variables|Default|GetActor%20ID)))
      (if _hasbeendestroyed
        (Actor|DestroyActor)))))

(fn ConstructionScript)