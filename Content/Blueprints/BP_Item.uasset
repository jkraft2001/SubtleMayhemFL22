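; BP_Item is a pickup actor that stays gone once collected, with the GameInstance tracking destroyed items.
; On BeginPlay it takes its display name as an ID and, after a short delay, destroys itself if already recorded.
; Collision overlap by any actor records the ID as destroyed.
; Only a BP_ThirdPersonCharacter overlap then triggers that character's SaveGame and removes the item.
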(event OnComponentBeginOverlap(Collision)
  (params (OverlappedComponent :type Primitive%20Component%20Object%20Reference) (OtherActor :type Actor%20Object%20Reference) (OtherComp :type Primitive%20Component%20Object%20Reference) (OtherBodyIndex :type Integer) (bFromSweep :type Boolean) (SweepResult :type Hit%20Result%20Structure%20%28by%20ref%29))
  (bind _asbp_game_instance (Utilities|Casting|CastToBP_GameInstance (Game|GetGameInstance)))
  (Default|DestroyItem _asbp_game_instance (Variables|Default|GetActorID))
  (bind _asbp_third_person_character (Utilities|Casting|CastToBP_ThirdPersonCharacter OtherActor))
  (Default|SaveGame _asbp_third_person_character)
  (Actor|DestroyActor))

(event EventBeginPlay
  (bind _output_get (Variables|Default|SetActorID (Utilities|String|StringToName (Utilities|GetDisplayName self))))
  (Utilities|FlowControl|Delay 0.2)
  (bind _asbp_game_instance (Utilities|Casting|CastToBP_GameInstance (Game|GetGameInstance)))
  (bind _hasbeendestroyed (Default|CheckifDestroyed _asbp_game_instance _output_get))
  (if _hasbeendestroyed
    (Actor|DestroyActor)))

(fn ConstructionScript)